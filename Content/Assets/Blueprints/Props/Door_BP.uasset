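; Physics-driven door prop that swings on a PhysicsConstraint and can be locked shut.
; SetLocked switches the constraint's Swing1 angular motion between Locked and Limited, then stores the state in the Locked variable.
; InteractWith only returns true, without moving the door or checking the lock.
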(event Custom|SetLocked
  (params (Lock :type Boolean))
  (bind _physicsconstraint (Variables|Default|GetPhysicsConstraint))
  (if Lock
    (Class|PhysicsConstraintComponent|SetAngularSwing1Limit _physicsconstraint "ACM_Locked" 9e+01)
    (else
      (Class|PhysicsConstraintComponent|SetAngularSwing1Limit _physicsconstraint "ACM_Limited" 9e+01)))
  (Variables|Default|SetLocked Lock))

(event EventBeginPlay
  (|CallParentFunction) ; This node is disabled and will not be called.\nDrag off pins to build functionality.
)

(event Collision|EventActorBeginOverlap
  (params (OtherActor :type Actor%20Object%20Reference))
  (|CallParentFunction OtherActor) ; This node is disabled and will not be called.\nDrag off pins to build functionality.
)

(event EventTick
  (params (DeltaSeconds :type Float%20%28single-precision%29))
  (|CallParentFunction DeltaSeconds) ; This node is disabled and will not be called.\nDrag off pins to build functionality.
)

(fn ConstructionScript
  (|CallParentFunction))

(fn Interactwith
  (params (Interactor :type Player%20BP%20Object%20Reference) (HitComponent :type Primitive%20Component%20Object%20Reference))
  (return true))