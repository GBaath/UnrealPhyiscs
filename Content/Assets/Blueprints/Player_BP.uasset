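; First-person player pawn that moves and looks via Enhanced Input and grabs physics objects by interacting with them.
; A per-tick camera trace finds simulating components implementing the interaction interface, outlines them with custom depth and shows their HUD message.
; Interact grabs through a PhysicsHandle that follows a GrabHandle each tick; release drops it.
; Locked doors show a coffee hint, and picking up or dropping KeyItems notifies the coffee machine.
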(event Input|EnhancedActionEvents|EnhancedInputActionCustomMove
  (params (ActionValue :type Vector%202D%20Structure) (ElapsedSeconds :type Float%20%28double-precision%29) (TriggeredSeconds :type Float%20%28double-precision%29) (InputAction :type Input%20Action%20Object%20Reference :default "/Game/Inputs/CustomMove.CustomMove"))
  ;[1 1 1] Move
  (:Triggered
    (Pawn|Input|AddMovementInput (Transformation|GetActorForwardVector) (.y ActionValue) false)
    (Pawn|Input|AddMovementInput (Transformation|GetActorRightVector) (.x ActionValue) false)))

(event Input|EnhancedActionEvents|EnhancedInputActionCustomLook
  (params (ActionValue :type Vector%202D%20Structure) (ElapsedSeconds :type Float%20%28double-precision%29) (TriggeredSeconds :type Float%20%28double-precision%29) (InputAction :type Input%20Action%20Object%20Reference :default "/Game/Inputs/CustomLook.CustomLook"))
  ;[1 1 1] Look
  (:Triggered
    (Pawn|Input|AddControllerYawInput (.x ActionValue))
    (Pawn|Input|AddControllerPitchInput (.y ActionValue))))

(event Input|EnhancedActionEvents|EnhancedInputActionCustomInteractRelease
  (params (ActionValue :type Boolean) (ElapsedSeconds :type Float%20%28double-precision%29) (TriggeredSeconds :type Float%20%28double-precision%29) (InputAction :type Input%20Action%20Object%20Reference :default "/Game/Inputs/CustomInteractRelease.CustomInteractRelease"))
  ;[1 1 1] release
  (:Triggered
    (if (CallFunction|IsHoldingObject)
      (Physics|Components|PhysicsHandle|ReleaseComponent (Variables|Default|GetPhysicsHandle))
      (Default|DisplayMsg (Variables|Default|GetHUDVar) "LEFT CLICK" 0.0)
      (Utilities|Casting|CastToKeyItem (Components|GetOwner (Variables|Default|GetLookAtComponent)))
      (Default|OnKeyItemDrop (Variables|Default|GetCoffeeMachine)))))

(event Input|EnhancedActionEvents|EnhancedInputActionCustomInteract
  (params (ActionValue :type Boolean) (ElapsedSeconds :type Float%20%28double-precision%29) (TriggeredSeconds :type Float%20%28double-precision%29) (InputAction :type Input%20Action%20Object%20Reference :default "/Game/Inputs/CustomInteract.CustomInteract"))
  (bind _physicshandle (Variables|Default|GetPhysicsHandle))
  ;[1 1 1] Grab Checks
  (:Triggered
    (bind _lookatcomponent (Variables|Default|GetLookAtComponent)
      (:then
        (bind _asdoor_bp (Utilities|Casting|CastToDoor_BP (Components|GetOwner _lookatcomponent))
          (:then
            (if (Variables|/Game/Assets/Blueprints/Props/Door_BP.Door_BP_C|GetLocked _asdoor_bp)
              (Default|DisplayMsg (Variables|Default|GetHUDVar) "I need coffee before I leave...." 1.0)
              (else
                (bind _cangrab (Class|FirstPersonInteractionsBPI|Interactwith(Message) (Components|GetOwner _lookatcomponent) self _lookatcomponent :!label _label))
                (if _cangrab
                  (if (CallFunction|IsHoldingObject)
                    (Physics|Components|PhysicsHandle|ReleaseComponent _physicshandle)
                    (else
                      (CallFunction|Grab 5e+02)
                      ;;[1 1 1] clear text on grab
                      (Default|DisplayMsg (Variables|Default|GetHUDVar) (Class|KismetTextLibrary|GetEmptyText) 0.0)
                      (Utilities|Casting|CastToKeyItem (Components|GetOwner _lookatcomponent))
                      (Default|OnKeyitemPickup (Variables|Default|GetCoffeeMachine))))
                  (else
                    (Physics|Components|PhysicsHandle|ReleaseComponent _physicshandle))))))
          (:CastFailed
            (goto _label))))
      (:else))))

(event EventBeginPlay
  (Utilities|FlowControl|Sequence
    (:then_0
      ;[1 1 1] HUD ref
      (bind _returnvalue (UserInterface|CreateWidget "/Game/Assets/Blueprints/UI_BP.UI_BP_C"))
      (bind _output_get (Variables|Default|SetHUDVar _returnvalue))
      (UserInterface|Viewport|AddtoViewport _output_get 0))
    (:then_1
      ;[1 1 1] add IMC Input
      (bind _asplayer_controller (Utilities|Casting|CastToPlayerController (Pawn|GetController)))
      (Input|AddMappingContext (PlayerController|LocalPlayerSubsystems|GetEnhancedInputLocalPlayerSubsystem _asplayer_controller) "/Game/Inputs/Custom_IMC.Custom_IMC" 0 "(bIgnoreAllPressedKeysUntilRelease=True,bForceImmediately=False)"))
    (:then_2
      ;[1 1 1] set refs
      (Utilities|FlowControl|Sequence
        (:then_0
          (bind _returnvalue_2 (Actor|GetActorOfClass "/Game/Assets/Blueprints/Props/Door_BP.Door_BP_C"))
          (Variables|Default|SetExitDoor _returnvalue_2))
        (:then_1
          (bind _returnvalue_3 (Actor|GetActorOfClass "/Game/Assets/Blueprints/Props/CoffeeMachine_BP.CoffeeMachine_BP_C"))
          (Variables|Default|SetCoffeeMachine _returnvalue_3))))))

(event Collision|EventActorBeginOverlap
  (params (OtherActor :type Actor%20Object%20Reference)))

(event EventTick
  (params (DeltaSeconds :type Float%20%28single-precision%29))
  (bind _grabhandle (Variables|Default|GetGrabHandle))
  (bind _returnvalue (Transformation|GetWorldTransform _grabhandle))
  (CallFunction|InteractionTrace 5e+02)
  ;[1 1 1] update grabbed if holding
  (if (CallFunction|IsHoldingObject)
    (Class|PhysicsHandleComponent|SetTargetLocationandRotation (Variables|Default|GetPhysicsHandle) (.location _returnvalue) (.rotation _returnvalue))))

(fn ConstructionScript)

(fn InteractionTrace
  (params (Range :type Float%20%28double-precision%29))
  (bind _camera (Variables|Default|GetCamera))
  (bind _returnvalue (Transformation|GetWorldLocation _camera))
  (if (not (CallFunction|IsHoldingObject))
    ;[1 1 1] Line from cam
    (bind (_outhit _returnvalue_2) (Collision|LineTraceByChannel _returnvalue (+ _returnvalue (* (Math|Vector|GetForwardVector (Variables|Default|GetCamera)) Range)) "TraceTypeQuery1" false 0 "None"))
    (if _returnvalue_2
      ;[1 1 1] Go thru if look at comp is different from previous
      (LocalVariables|SetLocalHitResults _outhit)
      (if (!= (Variables|Default|GetLookAtComponent) (.HitComponent (Collision|BreakHitResult _outhit)))
        (bind _lookatcomponent (Variables|Default|GetLookAtComponent)
          (:then
            (Rendering|SetRenderCustomDepth _lookatcomponent true))
          (:else
            _))
        (if (and (Utilities|DoesObjectImplementInterface (.HitActor (Collision|BreakHitResult _outhit)) "/Game/Assets/Blueprints/FirstPersonInteractions_BPI.FirstPersonInteractions_BPI_C") (Physics|IsSimulatingPhysics (.HitComponent (Collision|BreakHitResult _outhit)) "None"))
          ;[1 1 1] set new lookatcomp
          (bind (_lookatactor _lookatcomponent_2 _message) (Class|FirstPersonInteractionsBPI|Lookat(Message) (.HitActor (Collision|BreakHitResult (LocalVariables|GetLocalHitResults))) self (Game|GetPlayerController 0) (.HitComponent (Collision|BreakHitResult (LocalVariables|GetLocalHitResults)))))
          ;[1 1 1] Clear highlight
          (Rendering|SetRenderCustomDepth (Variables|Default|GetLookAtComponent) false)
          (Default|DisplayMsg (Variables|Default|GetHUDVar) (Class|KismetTextLibrary|GetEmptyText) 0.0)
          ;[1 1 1] Display msg and highlight
          (bind _output_get (Variables|Default|SetLookAtComponent _lookatcomponent_2))
          (Rendering|SetRenderCustomDepth _output_get true)
          (Default|DisplayMsg (Variables|Default|GetHUDVar) _message 0.0)
          (else
            ;[1 1 1] Clear highlight if not holding
            (if (not (CallFunction|IsHoldingObject)) :!label _label
              (bind _lookatcomponent_3 (Variables|Default|GetLookAtComponent)
                (:then
                  (Rendering|SetRenderCustomDepth _lookatcomponent_3 false)
                  (Default|DisplayMsg (Variables|Default|GetHUDVar) (Class|KismetTextLibrary|GetEmptyText) 0.0)
                  (Variables|Default|SetLookAtComponent 0))
                (:else))))))
      (else
        (goto _label)))))

(fn IsHoldingObject
  (return (Utilities|IsValid (Class|PhysicsHandleComponent|GetGrabbedComponent (Variables|Default|GetPhysicsHandle)))))

(fn Grab
  (params (Range :type Float%20%28double-precision%29))
  (bind _camera (Variables|Default|GetCamera))
  (bind _returnvalue (Transformation|GetWorldLocation _camera))
  (bind _outhit (Collision|LineTraceByChannel _returnvalue (+ _returnvalue (* (Math|Vector|GetForwardVector _camera) Range)) "TraceTypeQuery1" false 0 "None"))
  (Physics|Components|PhysicsHandle|GrabComponentatLocationwithRotation (Variables|Default|GetPhysicsHandle) (Variables|Default|GetLookAtComponent) "None" (.Location (Collision|BreakHitResult _outhit)) (Math|Rotator|MakeRotfromX (.Normal (Collision|BreakHitResult _outhit))))
  (Transformation|SetWorldLocationAndRotation (Variables|Default|GetGrabHandle) (.Location (Collision|BreakHitResult _outhit)) (Math|Rotator|MakeRotfromX (.Normal (Collision|BreakHitResult _outhit))) false false))