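; Lamp actor that the player can switch on and off when standing near it.
; Overlap events on a Trigger component set an Interactable flag while Player_BP is inside and clear it on exit.
; An interface Interact event toggles the PointLight's visibility only while that flag is set.
; On BeginPlay the lamp enables input from player controller 0.
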(event OnComponentBeginOverlap(Trigger)
  (params (OverlappedComponent :type Primitive%20Component%20Object%20Reference) (OtherActor :type Actor%20Object%20Reference) (OtherComp :type Primitive%20Component%20Object%20Reference) (OtherBodyIndex :type Integer) (bFromSweep :type Boolean) (SweepResult :type Hit%20Result%20Structure%20%28by%20ref%29))
  ;[1 1 1] Set Toggleability
  (Utilities|Casting|CastToPlayer_BP OtherActor)
  (Variables|Default|SetInteractable true))

(event OnComponentEndOverlap(Trigger)
  (params (OverlappedComponent :type Primitive%20Component%20Object%20Reference) (OtherActor :type Actor%20Object%20Reference) (OtherComp :type Primitive%20Component%20Object%20Reference) (OtherBodyIndex :type Integer))
  ;[1 1 1] Set Toggleability
  (Utilities|Casting|CastToPlayer_BP OtherActor)
  (Variables|Default|SetInteractable false))

(event EventBeginPlay
  (Input|EnableInput (Game|GetPlayerController 0)))

(event Collision|EventActorBeginOverlap
  (params (OtherActor :type Actor%20Object%20Reference)))

(event EventTick
  (params (DeltaSeconds :type Float%20%28single-precision%29)))

(event EventInteract
  ;[1 1 1] InteractEventFromInterface
  (if (Variables|Default|GetInteractable)
    (Rendering|ToggleVisibility (Variables|Default|GetPointLight) false)))

(fn ConstructionScript)